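; Base weapon Blueprint that plugs a weapon into its owner's Gameplay Ability System, caching the owner's ability component on BeginPlay.
; On equip it grants input-bound fire and alt abilities, storing their handles.
; It also applies GE_InitWeaponSet to the owner, passing Damage and FireRate as tagged SetByCaller magnitudes.
; On unequip it clears both abilities but leaves the applied effect untouched.
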(event `self.ReceiveBeginPlay`
  (set `self.OwnerASC` (`AbilitySystemBlueprintLibrary.GetAbilitySystemComponent` (`self.GetOwner`))))

(event `self.OnEquip`
  (bind _ownerasc (`self.OwnerASC`))
  (`KismetSystemLibrary.PrintString` "Weapon Equipped")
  (`|ExecutionSequence`
    (:`then_0`
      (bind _returnvalue (`AbilitySystemComponent.K2_GiveAbility` _ownerasc (`self.WeaponFireAbilityClass`) 0 (`KismetMathLibrary.Conv_ByteToInt` (`self.WeaponFireInputID`))))
      (set `self.WeaponFireAbilityHandle` _returnvalue))
    (:`then_1`
      (bind _returnvalue_2 (`AbilitySystemComponent.K2_GiveAbility` _ownerasc (`self.WeaponAltAbilityClass`) 0 (`KismetMathLibrary.Conv_ByteToInt` (`self.WeaponAltInputID`))))
      (set `self.WeaponAltAbilityHandle` _returnvalue_2))
    (:`then_2`
      (bind _returnvalue_3 (`AbilitySystemBlueprintLibrary.AssignTagSetByCallerMagnitude` (`AbilitySystemComponent.MakeOutgoingSpec` :`self` (`self.OwnerASC`) :`GameplayEffectClass` "/Game/Blueprints/GAS/Effects/GE_InitWeaponSet.GE_InitWeaponSet_C") (struct :`TagName` "WeaponSet.Init.Damage") (`self.Damage`)))
      (bind _returnvalue_4 (`AbilitySystemBlueprintLibrary.AssignTagSetByCallerMagnitude` _returnvalue_3 (struct :`TagName` "WeaponSet.Init.FireRate") (`self.FireRate`)))
      (`AbilitySystemComponent.BP_ApplyGameplayEffectSpecToSelf` (`self.OwnerASC`) _returnvalue_4))))

(event `self.OnUnEquip`
  (`KismetSystemLibrary.PrintString` "Weapon Unequipped")
  (`AbilitySystemComponent.ClearAbility` (`self.OwnerASC`) (`self.WeaponFireAbilityHandle`))
  (`AbilitySystemComponent.ClearAbility` (`self.OwnerASC`) (`self.WeaponAltAbilityHandle`)))

(fn `UserConstructionScript`)