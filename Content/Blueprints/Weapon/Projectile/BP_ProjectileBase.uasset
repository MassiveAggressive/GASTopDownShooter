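; BP_ProjectileBase is a base weapon projectile that deals damage on impact through the Gameplay Ability System.
; When its Box component hits an actor with an ability system component, the owner's component builds a GE_Damage spec and applies it to that target.
; The projectile's Damage value feeds the effect as a SetByCaller magnitude under the Damage.SetByCaller tag.
; The projectile destroys itself on any hit, whether or not damage is applied.
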(event `self.Box.OnComponentHit`
  (params (HitComponent :type "PrimitiveComponent Object Reference") (OtherActor :type "Actor Object Reference") (OtherComp :type "PrimitiveComponent Object Reference") (NormalImpulse :type "Vector Structure") (Hit :type "HitResult Structure (by ref)"))
  (bind _output_get (set `self.TargetASC` (`AbilitySystemBlueprintLibrary.GetAbilitySystemComponent` OtherActor)))
  (`/Engine/EditorBlueprintResources/StandardMacros.IsValid` _output_get
    (:`Is Valid`
      (bind _returnvalue (`AbilitySystemBlueprintLibrary.AssignTagSetByCallerMagnitude` (`AbilitySystemComponent.MakeOutgoingSpec` :`self` (`AbilitySystemBlueprintLibrary.GetAbilitySystemComponent` (`self.GetOwner`)) :`GameplayEffectClass` "/Game/Blueprints/GAS/Effects/GE_Damage.GE_Damage_C") (struct :`TagName` "Damage.SetByCaller") (`self.Damage`)))
      (`AbilitySystemComponent.BP_ApplyGameplayEffectSpecToTarget` (`AbilitySystemBlueprintLibrary.GetAbilitySystemComponent` (`self.GetOwner`)) _returnvalue (`self.TargetASC`))
      (`self.K2_DestroyActor`))
    (:`Is Not Valid`
      (`self.K2_DestroyActor`))))

(fn `UserConstructionScript`)