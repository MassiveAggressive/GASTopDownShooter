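; Gameplay Ability that fires the avatar character's weapon by spawning a projectile just in front of it, facing its rotation.
; Each shot commits the ability, and the projectile takes its damage from a gameplay attribute.
; Automatic weapons repeat through a WaitDelay loop timed by the inverse of an attribute value until input is released.
; Non-automatic weapons fire once and end the ability.
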(event `self.K2_ActivateAbility`
  (bind _asbp_third_person_character (cast `/Game/ThirdPerson/Blueprints/BP_ThirdPersonCharacter` (`self.GetAvatarActorFromActorInfo`)))
  (bind _output_get (set `self.AvatarActor` _asbp_third_person_character))
  (bind _output_get_2 (set `self.Weapon` (`TDSCharacter.Weapon` _output_get)))
  (set `self.IsAuto` (`TDSWeapon.IsAuto` _output_get_2))
  (`self.K2_CommitAbility`)
  (`self.Fire`)
  (if (`self.IsAuto`)
    (`AbilityTask_WaitInputRelease.WaitInputRelease` false
      (:`then`
        (`GameplayTask_WaitDelay.TaskWaitDelay` null (/ 1.0 (`.ReturnValue` (`AbilitySystemComponent.GetGameplayAttributeValue` (`AbilitySystemBlueprintLibrary.GetAbilitySystemComponent` (`self.AvatarActor`)) (struct :`AttributeName` "FireRate" :`Attribute` "/Script/TDS.TDSWeaponSet:FireRate" :`AttributeOwner` "/Script/CoreUObject.Class'/Script/TDS.TDSWeaponSet'")))) :!label _label
          (:`OnFinish`
            (`self.K2_CommitAbility`)
            (`self.Fire`)
            (goto _label))))
      (:`OnRelease`
        _)))
  (`self.K2_EndAbility`))

(fn `Fire`
  (bind _returnvalue (`self.GetAvatarActorFromActorInfo`))
  (`|SpawnActorFromClass` (`self.ProjectileClass`) (`KismetMathLibrary.MakeTransform` (+ (`Actor.K2_GetActorLocation` _returnvalue) (* (`Actor.GetActorForwardVector` _returnvalue) 25.0)) (`Actor.K2_GetActorRotation` _returnvalue)) "AlwaysSpawn" "MultiplyWithRoot" (`self.GetAvatarActorFromActorInfo`) (`.ReturnValue` (`AbilitySystemComponent.GetGameplayAttributeValue` (`AbilitySystemBlueprintLibrary.GetAbilitySystemComponent` (`self.GetAvatarActorFromActorInfo`)) (struct :`AttributeName` "Damage" :`Attribute` "/Script/TDS.TDSWeaponSet:Damage" :`AttributeOwner` "/Script/CoreUObject.Class'/Script/TDS.TDSWeaponSet'"))) null))